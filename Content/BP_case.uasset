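; BP_case is a board tile with a type (normal, casino, enemy, advance 2, back 2) and a displayed number.
; The construction script sets the number text and applies the material matching the tile type.
; It provides a separate world transform for each of four player IDs from spawn-location components, and Action returns the tile type to the caller.
; The BeginPlay switch on type has no effect, and leftover debug prints are unreachable.
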(event EventBeginPlay
  (switch Utilities|FlowControl|Switch|SwitchonE_CaseType (Variables|Default|GetCaseType)))

(fn ConstructionScript
  (Rendering|Components|TextRender|SetText (Variables|Default|GetTextRender) (Variables|Default|Gettextnum))
  (bind _material (CallFunction|GetMaterialConstruct))
  (Rendering|Material|SetMaterial (Variables|Default|Getcase) 0 _material))

(fn GetSocketPositionbyPlayerID
  (params (PlayerID :type Integer))
  (switch int PlayerID
    (:0
      (Variables|Default|SetLocationToReturn (Transformation|GetWorldTransform (Variables|Default|Getspawnloc1))))
    (:1
      (Variables|Default|SetLocationToReturn (Transformation|GetWorldTransform (Variables|Default|Getspawnloc2))))
    (:2
      (Variables|Default|SetLocationToReturn (Transformation|GetWorldTransform (Variables|Default|Getspawnloc3))))
    (:3
      (Variables|Default|SetLocationToReturn (Transformation|GetWorldTransform (Variables|Default|Getspawnloc4)))))
  (return (Variables|Default|GetLocationToReturn)))

(fn Action
  (return (Variables|Default|GetCaseType)))

(fn GetMaterialConstruct
  (switch Utilities|FlowControl|Switch|SwitchonE_CaseType (Variables|Default|GetCaseType)
    (:NewEnumerator0
      (Variables|Default|SetMaterial "/Game/Materials/Board/M_NormalCase.M_NormalCase"))
    (:NewEnumerator1
      (Variables|Default|SetMaterial "/Game/Materials/Board/M_CasinoCase.M_CasinoCase"))
    (:NewEnumerator2
      (Variables|Default|SetMaterial "/Game/Materials/Board/M_EnemyCase.M_EnemyCase"))
    (:NewEnumerator3
      (Variables|Default|SetMaterial "/Game/Materials/randomcolors/m_greeen.m_greeen"))
    (:NewEnumerator4
      (Variables|Default|SetMaterial "/Game/Materials/M_red.M_red")))
  (return (Variables|Default|GetMaterial)))