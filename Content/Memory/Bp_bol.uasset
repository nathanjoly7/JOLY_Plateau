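; Clickable piece, likely for a memory game, that opens and closes to reveal one of three element types.
; SetTypeFromNumber picks the Element mesh and matching enum, but BeginPlay always passes 0 and the random roll is unwired.
; Clicking Object_3 rolls Object2 via separate open and reversed close timelines, with Ismoving blocking clicks mid-animation.
; Visible tracks the open state, and the type is printed once opening finishes.
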(event OnClicked(Object_3)
  (params (TouchedComponent :type Primitive%20Component%20Object%20Reference) (ButtonPressed :type Key%20Structure :default "None"))
  (bind _object_2 (Variables|Default|GetObject_2))
  (bind _object_2_2 (Variables|Default|GetObject_2))
  (bind _relativerotation (Variables|/Script/Engine.SceneComponent|GetRelativeRotation _object_2))
  (bind _relativerotation_2 (Variables|/Script/Engine.SceneComponent|GetRelativeRotation _object_2_2))
  (if (not (Variables|Default|Getismoving))
    (if (Variables|Default|GetVisible)
      (Variables|Default|Setismoving true)
      (bind _newtrack_0 (Timeline|Timeline_0 ReverseFromEnd)
        (:Update
          (Transformation|SetRelativeRotation _object_2 (Math|Rotator|MakeRotator _newtrack_0 (.pitch _relativerotation) (.yaw _relativerotation)) false false))
        (:Finished
          (Variables|Default|SetVisible false)
          (Variables|Default|Setismoving false)))
      (else
        ;[1 1 1] Open
        (Variables|Default|Setismoving true)
        (bind _newtrack_0_2 (Timeline|Timeline PlayFromStart)
          (:Update
            (Transformation|SetRelativeRotation _object_2_2 (Math|Rotator|MakeRotator _newtrack_0_2 (.pitch _relativerotation_2) (.yaw _relativerotation_2)) false false))
          (:Finished
            (Variables|Default|SetVisible true)
            (Variables|Default|Setismoving false)
            (Development|PrintString (Utilities|String|EnumtoString (Variables|Default|GetType)))))))))

(event EventBeginPlay
  (CallFunction|SetTypefromNumber))

(fn ConstructionScript)

(fn SetTypefromNumber
  (params (number :type Integer))
  (Components|StaticMesh|SetStaticMesh (Variables|Default|Getelement) (Utilities|Array|Get(acopy) (Variables|Default|GetMeshes) number))
  (switch int number
    (:0
      (Variables|Default|SetType "NewEnumerator0"))
    (:1
      (Variables|Default|SetType "NewEnumerator1"))
    (:2
      (Variables|Default|SetType "NewEnumerator2")))
  (return (Variables|Default|GetType) number))