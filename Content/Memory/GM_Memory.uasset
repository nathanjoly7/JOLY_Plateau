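; Game mode for a Memory minigame where bowls are matched in pairs within a limited number of attempts.
; BeginPlay shuffles the type list onto all Bp_bol actors, enables mouse clicks and creates the WB_Memory HUD.
; CheckCard compares successive bowls, destroying matches or resetting mismatches, with sound and score feedback.
; When attempts run out, GameOver adds the pairs to player 1's GI_main score, regardless of starting player, and opens Level1.
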(event Custom|GameOver
  (bind _as_gi_main (Variables|Default|GetAs%20GI%20Main))
  (bind _pointsvictoire (Default|GetScorebyPlayerID _as_gi_main 1))
  (Default|SetScorebyPlayerID _as_gi_main 1 (+ _pointsvictoire (Variables|Default|GetPaires)))
  (Utilities|FlowControl|Delay 1.0)
  (Game|OpenLevel(byObjectReference) "/Game/Level1.Level1"))

(event EventBeginPlay
  (bind _returnvalue (Game|GetPlayerController 0))
  (Utilities|FlowControl|Sequence
    (:then_0
      (Utilities|Array|Shuffle (Variables|Default|GetListe%20des%20types%20a%20avoir))
      (Utilities|FlowControl|Delay 0.2)
      (Variables|/Script/Engine.PlayerController|SetbEnableClickEvents _returnvalue true)
      (Variables|/Script/Engine.PlayerController|SetbShowMouseCursor _returnvalue true)
      (bind _outactors (Actor|GetAllActorsOfClass "/Game/Memory/Bp_bol.Bp_bol_C"))
      (bind _output_get (Variables|Default|SetListeBols _outactors))
      (for (_array_element _array_index) _output_get
        (bind _numberr (Default|SetTypefromNumber _array_element (Utilities|Array|Get(acopy) (Variables|Default|GetListe%20des%20types%20a%20avoir) _array_index)))))
    (:then_1
      (bind _asgi_main (Utilities|Casting|CastToGI_main (Game|GetGameInstance)))
      (Variables|Default|SetAs%20GI%20Main _asgi_main))
    (:then_2
      (bind _returnvalue_2 (UserInterface|CreateWidget "/Game/UI/WB_Memory.WB_Memory_C"))
      (Variables|Default|Setwidgethud _returnvalue_2)
      (UserInterface|Viewport|AddtoViewport _returnvalue_2 0)
      (Utilities|FlowControl|Delay 0.7)
      (Rendering|Components|TextRender|SetText (Variables|/Game/UI/WB_Memory.WB_Memory_C|Gettextplayer _returnvalue_2) (Utilities|Text|FormatText "Player :{p}" (Variables|Default|GetPlayerWhoStartedGame)))
      (Rendering|Components|TextRender|SetText (Variables|/Game/UI/WB_Memory.WB_Memory_C|Gettextscore (Variables|Default|Getwidgethud)) (Utilities|Text|FormatText "Paires : {p}" (Variables|Default|GetPaires))))))

(event EventTick
  (params (DeltaSeconds :type Float%20%28single-precision%29)))

(fn ConstructionScript)

(fn CheckCard
  (params (bol :type Bp%20Bol%20Object%20Reference))
  (bind _essais_restants (Variables|Default|GetEssais%20restants))
  (if (Utilities|IsValid (Variables|Default|GetPreviousBol))
    (Math|Integer|DecrementInt _essais_restants
      (:%20%20
        (if (> _essais_restants 0)
          (Development|PrintText (Utilities|Text|FormatText "ESSAIS RESTANTS : {e}" _essais_restants) true true "(R=1.000000,G=0.265081,B=0.084755,A=1.000000)")
          (if (Utilities|Enum|Equal(Enum) (Variables|/Game/Memory/Bp_bol.Bp_bol_C|GetType bol) (Variables|/Game/Memory/Bp_bol.Bp_bol_C|GetType (Variables|Default|GetPreviousBol)))
            (Actor|DestroyActor bol)
            (bind _result (Math|Integer|IncrementInt (Variables|Default|GetPaires))
              (:%20%20
                (Development|PrintString (Utilities|String|ToString(Integer) _result))
                (Audio|PlaySound2D "/Game/Sound/arcade-ui-14-229514.arcade-ui-14-229514" 1.0 1.0 0.0 0 0)
                (Rendering|Components|TextRender|SetText (Variables|/Game/UI/WB_Memory.WB_Memory_C|Gettextscore (Variables|Default|Getwidgethud)) (Utilities|Text|FormatText "Paires : {p}" (Variables|Default|GetPaires)))))
            (else
              (Default|ResetBol bol)
              (Variables|Default|SetPreviousBol 0)
              (Audio|PlaySound2D "/Engine/EditorSounds/Notifications/CompileFailed.CompileFailed" 1.0 1.0 0.0 0 0)))
          (else
            (Development|PrintString "GAME OVER" true true "(R=1.000000,G=0.047707,B=0.000000,A=1.000000)")
            (CallFunction|GameOver)))))
    (else
      (Variables|Default|SetPreviousBol bol))))

(fn SetPlayer
  (params (PlayerWhoStartedGame :type Integer))
  (Variables|Default|SetPlayerWhoStartedGame PlayerWhoStartedGame))