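; BP_cube is an actor that tints its cube and repeatedly spawns BP_projtest projectile actors from its Sphere component.
; On BeginPlay it creates a dynamic MI_black instance and, after a one-second delay, sets its BaseColor to the Colorr variable.
; Tick runs through a short Delay that throttles spawning to roughly five per second.
; An alternate projectile spawn, a red material swap and a RadialForce reference are left unused.
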(event EventTick
  (params (DeltaSeconds :type Float%20%28single-precision%29))
  (Utilities|FlowControl|Delay 0.2)
  (Game|SpawnActorfromClass "/Game/Vrac/BP_projtest.BP_projtest_C" (Transformation|GetWorldTransform (Variables|Default|GetSphere)) "Undefined" "MultiplyWithRoot" 0 0))

(event EventBeginPlay
  (bind _returnvalue (Rendering|Material|CreateDynamicMaterialInstance (Variables|Default|GetCube) 0 "/Game/Materials/MI_black.MI_black" "None" :!class /Script/Engine.PrimitiveComponent))
  (Variables|Default|SetDMI_cube _returnvalue)
  (Utilities|FlowControl|Delay 1.0)
  (CallFunction|ChangeColor))

(fn ConstructionScript)

(fn ChangeColor
  (Rendering|Material|SetVectorParameterValue (Variables|Default|GetDMI_cube) "BaseColor" (Variables|Default|Getcolorr) :!class /Script/Engine.MaterialInstanceDynamic))