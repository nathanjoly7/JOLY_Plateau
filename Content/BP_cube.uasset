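; BP_cube is an actor with Cube and Sphere components that recolors its cube shortly after play begins.
; BeginPlay creates a dynamic material instance from M_black on the Cube, then after a short delay calls ChangeColor to set its BaseColor parameter from the Colorr variable.
; Leftover unconnected nodes for spawning BP_projtest at the Sphere and applying M_red never run.
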(event EventTick
  (params (DeltaSeconds :type Float%20%28single-precision%29)))

(event EventBeginPlay
  (bind _returnvalue (Rendering|Material|CreateDynamicMaterialInstance (Variables|Default|GetCube) 0 "/Game/M_black.M_black" "" :!class /Script/Engine.PrimitiveComponent))
  (Variables|Default|SetDMI_cube _returnvalue)
  (Utilities|FlowControl|Delay 1.0)
  (CallFunction|ChangeColor))

(fn ConstructionScript)

(fn ChangeColor
  (Rendering|Material|SetVectorParameterValue (Variables|Default|GetDMI_cube) "BaseColor" (Variables|Default|Getcolorr) :!class /Script/Engine.MaterialInstanceDynamic))