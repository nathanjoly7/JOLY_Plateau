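; Player Blueprint that handles the dice-roll input for a turn-based, multiplayer dice-and-move game.
; BeginPlay caches the GM_main game mode and GI_main game instance.
; Pressing E asks the game mode to roll and move the current player, locking input behind a two-second delay.
; It then clears all widgets and advances the player ID, wrapping around the game instance's player list; leftover test nodes are disconnected.
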(event EventBeginPlay
  (bind _asgm_main (Utilities|Casting|CastToGM_main (Game|GetGameMode)))
  (Variables|Default|SetAs%20GM%20Main _asgm_main)
  (bind _asgi_main (Utilities|Casting|CastToGI_main (Game|GetGameInstance)))
  (Variables|Default|SetAs%20GI%20Main _asgi_main))

(event Input|KeyboardEvents|E
  (params (Key :type Key%20Structure :default "None"))
  (:Pressed
    (if (Variables|Default|Getcanrolldice)
      (Default|RollDiceandMove (Variables|Default|GetAs%20GM%20Main) (Variables|Default|GetPlayer0ToPlay) (Variables|Default|Getplayeridtoplay))
      (Variables|Default|Setcanrolldice false)
      (Utilities|FlowControl|Delay 2.0)
      (Development|PrintString "Can roll")
      (Variables|Default|Setcanrolldice true)
      (Viewport|RemoveAllWidgets)
      ;[1 1 1] si il y a d'autres joueurs passer au joueur +1 sinon reset
      (if (> (- (Utilities|Array|Length (Variables|/Game/GI_main.GI_main_C|Getst%20player%20list (Variables|Default|GetAs%20GI%20Main))) 1) (Variables|Default|Getplayeridtoplay))
        (Math|Integer|IncrementInt (Variables|Default|Getplayeridtoplay))
        (else
          (Variables|Default|Setplayeridtoplay 0))))))

(event Input|KeyboardEvents|A
  (params (Key :type Key%20Structure :default "None")))

(fn ConstructionScript)