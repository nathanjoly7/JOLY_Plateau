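; BP_Board is a game board Blueprint that maps a cell index and player ID to a world transform.
; GetCellPositionByIndex looks up the cell in CaseList and returns one of its four spawn-point transforms, one for each player.
; A chain that would register the board with GM_main is disconnected, so BeginPlay and the construction script do nothing.
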(event EventBeginPlay)

(fn ConstructionScript)

(fn GetCellPositionbyIndex
  (params (Index :type Integer) (PlayerID :type Integer))
  (bind _caselist (Variables|Default|GetCaseList))
  (bind _output (Utilities|Array|Get(acopy) _caselist Index))
  (switch int PlayerID
    (:0
      (return (Transformation|GetWorldTransform (Variables|/Game/BP_case.BP_case_C|Getspawnloc1 _output))))
    (:1
      (return (Transformation|GetWorldTransform (Variables|/Game/BP_case.BP_case_C|Getspawnloc2 _output))))
    (:2
      (return (Transformation|GetWorldTransform (Variables|/Game/BP_case.BP_case_C|Getspawnloc3 _output))))
    (:3
      (return (Transformation|GetWorldTransform (Variables|/Game/BP_case.BP_case_C|Getspawnloc4 _output))))))