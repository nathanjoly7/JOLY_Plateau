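; Main game mode for a dice-driven board race between two players, won by reaching cell 13.
; BeginPlay finds the board, spawns a pawn per player stored in GI_main, and spawns the dice.
; RollDiceAndMove rolls for either player and caps the target at 13; Move1by1 recursively advances the pawn cell by cell with short delays, updating GI_main.
; Reaching the last cell shows the victory widget, then quits the game.
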(event Custom|GetCaseLoc
  (params (caseindex :type Integer))
  ;[1 1 1] ma version
  (CallFunction|SpawnPion (Transformation|GetWorldTransform (Variables|/Game/BP_case.BP_case_C|Getspawnloc1 (Utilities|Array|Get(acopy) (Variables|/Game/BP_Board.BP_Board_C|GetCaseList (Variables|Default|Getboard)) caseindex)))))

(event Custom|SpawnPion
  (params (loc :type Transform))
  ;[1 1 1] ma version
  (Game|SpawnActorfromClass "/Game/BP_Pion.BP_Pion_C" loc "AdjustIfPossibleButAlwaysSpawn" "MultiplyWithRoot" 0 0))

(event Custom|NewSpawnPion
  (params (player%20ID :type Integer))
  (bind _as_gi_main (Variables|Default|GetAs%20GI%20Main))
  (Default|GetCellNumberbyPlayerID _as_gi_main player%20ID)
  (bind _positioncase (Default|GetCellPositionbyIndex (Variables|Default|Getboard) (Variables|/Game/GI_main.GI_main_C|GetSt%20Player%20Case%20Index _as_gi_main) player%20ID))
  (bind _returnvalue (Game|SpawnActorfromClass "/Game/BP_Pion.BP_Pion_C" (Math|Transform|MakeTransform (.location _positioncase) (.rotation _positioncase) (.scale _positioncase)) "AdjustIfPossibleButAlwaysSpawn" "MultiplyWithRoot" 0 0))
  (bind _output_get (Variables|Default|SetPion _returnvalue))
  (Utilities|Array|Add (Variables|Default|GetListPions) _output_get)
  (Variables|Default|SetIsAlreadySpawned true))

(event Custom|RollDiceAndMove1by1
  (bind _output_dice_number (Default|RollDice (Variables|Default|Getbp_dice) false))
  (bind _caseindex (Default|GetCellNumberbyPlayerID (Variables|Default|GetAs%20GI%20Main)))
  (if (> (+ _caseindex _output_dice_number) 13)
    (Variables|Default|SetTargetCaseIndex (- (+ _caseindex _output_dice_number) 13))
    (else
      (bind _output_get (Variables|Default|SetTargetCaseIndex (+ _caseindex _output_dice_number)))))
  (bind _caseindex_2 (Default|GetCellNumberbyPlayerID (Variables|Default|GetAs%20GI%20Main))))

(event Custom|Move1by1
  (params (target%20case%20index :type Integer) (PlayerID :type Integer))
  (bind _result (Utilities|Text|FormatText "Victoire Player {id}" PlayerID))
  (if (Math|Integer|InRange(Integer) target%20case%20index 1 13)
    (bind _caseindex (Default|GetCellNumberbyPlayerID (Variables|Default|GetAs%20GI%20Main) PlayerID))
    (bind _caseindex_2 (Default|GetCellNumberbyPlayerID (Variables|Default|GetAs%20GI%20Main) PlayerID))
    (if (< _caseindex target%20case%20index)
      (Default|SetPlayerCellNumberbyPlayerID (Variables|Default|GetAs%20GI%20Main) (+ _caseindex_2 1) PlayerID)
      (bind _positioncase (Default|GetCellPositionbyIndex (Variables|Default|Getboard) (+ _caseindex_2 1) PlayerID))
      (Default|MovetoNewCell (Utilities|Array|Get(acopy) (Variables|Default|GetListPions) PlayerID) (.location _positioncase) (.rotation _positioncase))
      (bind _caseindex_3 (Default|GetCellNumberbyPlayerID (Variables|Default|GetAs%20GI%20Main) PlayerID))
      (if (== _caseindex_3 13)
        (Variables|Default|SetGameOver true)
        (Development|PrintText _result)
        (Utilities|FlowControl|Delay 0.5)
        (bind _returnvalue (UserInterface|CreateWidget "/Game/UI/WB_GameOver.WB_GameOver_C"))
        (UserInterface|Viewport|AddtoViewport _returnvalue 0)
        (Rendering|Components|TextRender|SetText (Variables|/Game/UI/WB_GameOver.WB_GameOver_C|GetTextBlock_0 _returnvalue) _result)
        (Utilities|FlowControl|Delay 5.0)
        (Game|QuitGame 0 "Quit" false)
        (else
          (Utilities|FlowControl|Delay 0.2)
          (CallFunction|Move1by1 target%20case%20index PlayerID)))
      (else
        (Variables|Default|SetTargetCaseIndex 0)))
    (else
      (bind _positioncase_2 (Default|GetCellPositionbyIndex (Variables|Default|Getboard)))
      (Default|MovetoNewCell (Variables|Default|GetPion) (.location _positioncase_2) (.rotation _positioncase_2)))))

(event EventBeginPlay
  (bind _returnvalue (Actor|GetActorOfClass "/Game/BP_Board.BP_Board_C"))
  (Variables|Default|Setboard _returnvalue)
  (bind _asgi_main (Utilities|Casting|CastToGI_main (Game|GetGameInstance)))
  (bind _output_get (Variables|Default|SetAs%20GI%20Main _asgi_main))
  (for _array_element (Variables|/Game/GI_main.GI_main_C|Getst%20player%20list _output_get)
    (CallFunction|NewSpawnPion (.playerID (Utilities|Struct|BreakST_Player _array_element))))
  (bind _returnvalue_2 (Game|SpawnActorfromClass "/Game/BP_dice.BP_dice_C" (Math|Transform|MakeTransform "0, 0, 0") "Undefined" "MultiplyWithRoot" 0 0))
  (Variables|Default|Setbp_dice _returnvalue_2))

(event EventTick
  (params (DeltaSeconds :type Float%20%28single-precision%29)))

(fn ConstructionScript)

(fn RollDiceandMove
  (params (Player0 :type Boolean))
  (if (not (Variables|Default|GetGameOver))
    (if Player0
      ;[1 1 1] version move1by1
      (bind _output_dice_number (Default|RollDice (Variables|Default|Getbp_dice) Player0))
      (bind _caseindex (Default|GetCellNumberbyPlayerID (Variables|Default|GetAs%20GI%20Main)))
      (if (> (+ _caseindex _output_dice_number) 13)
        (Development|PrintString ">13")
        (bind _output_get (Variables|Default|SetTargetCaseIndex 13))
        (CallFunction|Move1by1 _output_get)
        (else
          (bind _output_get_2 (Variables|Default|SetTargetCaseIndex (+ _caseindex _output_dice_number)))
          (CallFunction|Move1by1 _output_get_2)))
      (else
        ;[1 1 1] ID1
        (bind _output_dice_number_2 (Default|RollDice (Variables|Default|Getbp_dice) Player0))
        (bind _caseindex_2 (Default|GetCellNumberbyPlayerID (Variables|Default|GetAs%20GI%20Main) 1))
        (if (> (+ _caseindex_2 _output_dice_number_2) 13)
          (Development|PrintString ">13")
          (bind _output_get_3 (Variables|Default|SetTargetCaseIndex 13))
          (CallFunction|Move1by1 _output_get_3 1)
          (else
            (bind _output_get_4 (Variables|Default|SetTargetCaseIndex (+ _caseindex_2 _output_dice_number_2)))
            (CallFunction|Move1by1 _output_get_4 1)))))))