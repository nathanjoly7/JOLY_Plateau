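; BP_De is a dice-rolling Blueprint that shows random results in a WB_Dice widget.
; Five seconds after BeginPlay it raises a flag and adds the widget to the viewport.
; While the flag is set, Tick uses a Delay as a 0.4-second throttle to repeatedly call RollDice.
; RollDice sums zero-based random integers over DicesToRoll, and the total selects the widget switcher's active page.
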(event EventBeginPlay
  (Utilities|FlowControl|Delay 5.0)
  (Variables|Default|SetNewVar true)
  (bind _returnvalue (UserInterface|CreateWidget "/Game/UI/WB_Dice.WB_Dice_C"))
  (bind _output_get (Variables|Default|SetWidgetDe _returnvalue))
  (UserInterface|Viewport|AddtoViewport _output_get 0))

(event EventTick
  (params (DeltaSeconds :type Float%20%28single-precision%29))
  (if (Variables|Default|GetNewVar)
    (Utilities|FlowControl|Delay 0.4)
    (bind _output_get (CallFunction|RollDice))
    (Class|WidgetSwitcher|SetActiveWidgetIndex (Variables|/Game/UI/WB_Dice.WB_Dice_C|GetWidgetSwitcher_0 (stale EventBeginPlay _output_get)) _output_get)))

(fn ConstructionScript)

(fn RollDice
  (Variables|Default|SetDiceResult 0)
  (for _index (range 0 (- (Variables|Default|GetDices%20to%20roll) 1))
    (Variables|Default|SetDiceResult (+ (Variables|Default|GetDiceResult) (Math|Random|RandomIntegerinRange 0 (Variables|Default|GetMax)))))
  (return (Variables|Default|GetDiceResult)))