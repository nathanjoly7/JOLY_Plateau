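; Dice Blueprint for a board game that rolls for a player and shows the result on screen.
; On BeginPlay, after a short delay and if rolling is allowed, it creates the WB_Dice widget and caches the GM_main game mode.
; RollDice sums random rolls, sets the widget's face and player-specific text through widget switchers, and returns the sum plus one.
; Older roll-trigger and pawn-movement logic remains in the EventGraph, disconnected.
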(event EventBeginPlay
  (Utilities|FlowControl|Delay 1.0)
  (if (Variables|Default|Getcanrolldice)
    (bind _returnvalue (UserInterface|CreateWidget "/Game/UI/WB_Dice.WB_Dice_C"))
    (bind _output_get (Variables|Default|SetWidgetDe _returnvalue))
    (bind _asgm_main (Utilities|Casting|CastToGM_main (Game|GetGameMode)))
    (Variables|Default|SetAs%20GM%20Main _asgm_main)))

(event EventTick
  (params (DeltaSeconds :type Float%20%28single-precision%29)))

(fn ConstructionScript)

(fn RollDice
  (params (IsPlayer0 :type Boolean))
  (Variables|Default|SetDiceResult 0)
  (for _index (range 0 (- (Variables|Default|GetDices%20to%20roll) 1))
    (Variables|Default|SetDiceResult (+ (Variables|Default|GetDiceResult) (Math|Random|RandomIntegerinRange 1 (Variables|Default|GetMax)))))
  (UserInterface|Viewport|AddtoViewport (Variables|Default|GetWidgetDe) 0)
  (Class|WidgetSwitcher|SetActiveWidgetIndex (Variables|/Game/UI/WB_Dice.WB_Dice_C|GetWidgetSwitcher_0 (Variables|Default|GetWidgetDe)) (Variables|Default|GetDiceResult))
  (if IsPlayer0
    (Class|WidgetSwitcher|SetActiveWidgetIndex (Variables|/Game/UI/WB_Dice.WB_Dice_C|GetWidgetSwitcherTEXT (Variables|Default|GetWidgetDe)))
    (else
      (Class|WidgetSwitcher|SetActiveWidgetIndex (Variables|/Game/UI/WB_Dice.WB_Dice_C|GetWidgetSwitcherTEXT (Variables|Default|GetWidgetDe)) 1)))
  (Development|PrintString (Utilities|String|ToString(Text) (Utilities|Text|FormatText "Dice Result : {d}" (+ (Variables|Default|GetDiceResult) 1))))
  (return (+ (Variables|Default|GetDiceResult) 1)))