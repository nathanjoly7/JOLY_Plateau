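; BP_Laser is a laser actor that sweeps back and forth horizontally by oscillating its yaw.
; Each tick steps the actor's yaw by one degree, keeping pitch and roll unchanged.
; The Gootherway boolean flips the direction when yaw reaches either end of a fixed arc centered on zero.
; The step ignores delta time, so sweep speed depends on frame rate.
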(event EventBeginPlay)

(event EventTick
  (params (DeltaSeconds :type Float%20%28single-precision%29))
  (bind _returnvalue (Transformation|GetActorRotation))
  (if (Variables|Default|Getgootherway)
    (bind _result (Math|Float|DecrementFloat (.yaw _returnvalue))
      (:%20%20
        (if (<= _result -8e+01)
          (Variables|Default|Setgootherway false))
        (Transformation|SetActorRotation (Math|Rotator|MakeRotator (.roll _returnvalue) (.pitch _returnvalue) _result))))
    (else
      (bind _result_2 (Math|Float|IncrementFloat (.yaw _returnvalue))
        (:%20%20
          (if (>= _result_2 8e+01)
            (Variables|Default|Setgootherway true))
          (Transformation|SetActorRotation (Math|Rotator|MakeRotator (.roll _returnvalue) (.pitch _returnvalue) _result_2)))))))

(fn ConstructionScript)